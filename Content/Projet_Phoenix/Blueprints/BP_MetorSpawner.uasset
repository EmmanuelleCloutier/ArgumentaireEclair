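; Meteor spawner actor that periodically launches BP_Meteor actors aimed at the boat.
; On BeginPlay it rotates toward TargetActor and starts a looping timer, with an interval randomized once between SpawnInterval and a fixed maximum.
; Each tick of that timer has a one-in-seven chance to spawn a meteor at the spawner's root transform.
; The meteor gets a random star or holes mesh and receives the BP_Boat target.
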(event EventBeginPlay
  (bind _returnvalue (Transformation|GetActorLocation))
  (bind _targetactor (Variables|Default|GetTargetActor))
  (bind _returnvalue_2 (Transformation|GetActorLocation _targetactor))
  (bind _returnvalue_3 (- _returnvalue_2 _returnvalue))
  (bind _returnvalue_4 (Math|Vector|Normalize _returnvalue_3))
  (Transformation|SetActorRotation (Math|Rotator|MakeRotationfromAxes _returnvalue_4 _returnvalue_4 _returnvalue_4))
  (Utilities|Time|SetTimerbyFunctionName 0 "Spawn Meteor" (Math|Random|RandomFloatinRange (Variables|Default|GetSpawnInterval) 2e+01) true))

(fn ConstructionScript)

(fn SpawnMeteor
  (switch int (Math|Random|RandomInteger 7)
    (:0
      (bind _returnvalue (Game|SpawnActorfromClass "/Game/Projet_Phoenix/Blueprints/BP_Meteor.BP_Meteor_C" (Transformation|GetRelativeTransform (Variables|Default|GetDefaultSceneRoot)) "AlwaysSpawn" "MultiplyWithRoot" 0 0))
      (if (== (Math|Random|RandomInteger 4) 1)
        (Components|StaticMesh|SetStaticMesh (Variables|/Game/Projet_Phoenix/Blueprints/BP_Meteor.BP_Meteor_C|GetBaseMesh _returnvalue) "/Game/Mesh/SM_Meteorite_star.SM_Meteorite_star")
        (else
          (Components|StaticMesh|SetStaticMesh (Variables|/Game/Projet_Phoenix/Blueprints/BP_Meteor.BP_Meteor_C|GetBaseMesh _returnvalue) "/Game/Mesh/SM_Meteorite_holes.SM_Meteorite_holes")))
      (bind _asbp_boat (Utilities|Casting|CastToBP_Boat (Variables|Default|GetTargetActor)))
      (Variables|/Game/Projet_Phoenix/Blueprints/BP_Meteor.BP_Meteor_C|SetTarget _returnvalue _asbp_boat))))