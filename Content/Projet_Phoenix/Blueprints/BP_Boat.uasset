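; BP_Boat is the boat actor that takes damage and triggers the death screen when its life runs out.
; On BeginPlay it caches the world positions of three damage location components.
; Each Damage event spawns a BP_Damage at a random cached position, ignoring the passed HitLocation, then subtracts fixed life and prints it.
; At zero life it shows WBP_Death with UI-only input and the mouse cursor.
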(event Custom|Damage
  (params (Hit%20location :type Vector))
  (bind _returnvalue (Game|GetPlayerController 0))
  (Game|SpawnActorfromClass "/Game/Projet_Phoenix/Blueprints/BP_Damage.BP_Damage_C" (Math|Transform|MakeTransform (.OutItem (Utilities|Array|Random (Variables|Default|GetPossibleDamageLocation))) "0, 0, 0" "1.000000,1.000000,1.000000") "Undefined" "MultiplyWithRoot" 0 0)
  (bind _output_get (Variables|Default|SetLife (- (Variables|Default|GetLife) 5e+01)))
  (Development|PrintString (Utilities|String|ToString(Float) _output_get))
  (if (<= _output_get 0.0)
    (bind _returnvalue_2 (UserInterface|CreateWidget "/Game/Projet_Phoenix/Blueprints/WBP_Death.WBP_Death_C"))
    (bind _output_get_2 (Variables|Default|SetDeathWidget _returnvalue_2))
    (UserInterface|Viewport|AddtoViewport _output_get_2 0)
    (Input|SetInputModeUIOnly _returnvalue _output_get_2 "DoNotLock" false)
    (Variables|/Script/Engine.PlayerController|SetbShowMouseCursor _returnvalue true)))

(event EventBeginPlay
  (Utilities|Array|Add (Variables|Default|GetPossibleDamageLocation) (Transformation|GetWorldLocation (Variables|Default|GetDamageLocation_1)))
  (Utilities|Array|Add (Variables|Default|GetPossibleDamageLocation) (Transformation|GetWorldLocation (Variables|Default|GetDamageLocation_2)))
  (Utilities|Array|Add (Variables|Default|GetPossibleDamageLocation) (Transformation|GetWorldLocation (Variables|Default|GetDamageLocation_3))))

(fn ConstructionScript)