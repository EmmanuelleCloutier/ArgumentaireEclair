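; BP_Damage is a repairable damage spot that registers in the player character's damage list and snaps onto the boat with a downward trace.
; Its box overlap hands itself to the player, or slows an attacking companion and shows its repair kit and a progress bar.
; After TimeToFix, a timer removes it from the list, then resets the companion and destroys the actor.
; Tick turns the prompt and active progress bar toward the camera.
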(event OnComponentBeginOverlap(Box)
  (params (OverlappedComponent :type Primitive%20Component%20Object%20Reference) (OtherActor :type Actor%20Object%20Reference) (OtherComp :type Primitive%20Component%20Object%20Reference) (OtherBodyIndex :type Integer) (bFromSweep :type Boolean) (SweepResult :type Hit%20Result%20Structure%20%28by%20ref%29))
  (bind _asbp_third_person_character (Utilities|Casting|CastToBP_ThirdPersonCharacter OtherActor)
    (:then
      (Variables|/Game/ThirdPerson/Blueprints/BP_ThirdPersonCharacter.BP_ThirdPersonCharacter_C|SetBoatDamage _asbp_third_person_character self))
    (:CastFailed
      (bind _asbp_companion (Utilities|Casting|CastToBP_Companion OtherActor))
      (if (Variables|/Game/Blueprints/BP_Companion.BP_Companion_C|GetisAttacking _asbp_companion)
        (Utilities|Time|SetTimerbyEvent (delegate Custom|DestroyActor) (Variables|Default|GetTimeToFix))
        (Variables|/Script/Engine.ProjectileMovementComponent|SetMaxSpeed (Variables|/Game/Blueprints/BP_Companion.BP_Companion_C|GetProjectileMovement _asbp_companion) 0.1)
        (CallFunction|StartRepairing)
        (Rendering|SetVisibility (Variables|/Game/Blueprints/BP_Companion.BP_Companion_C|Getrepair%20kit _asbp_companion) true false)
        (Utilities|FlowControl|Delay (Variables|Default|GetTimeToFix))
        (Rendering|SetVisibility (Variables|/Game/Blueprints/BP_Companion.BP_Companion_C|Getrepair%20kit _asbp_companion) false false)
        (else
          (Rendering|SetVisibility (Variables|/Game/Blueprints/BP_Companion.BP_Companion_C|Getrepair%20kit _asbp_companion) false false))))))

(event OnComponentEndOverlap(Box)
  (params (OverlappedComponent :type Primitive%20Component%20Object%20Reference) (OtherActor :type Actor%20Object%20Reference) (OtherComp :type Primitive%20Component%20Object%20Reference) (OtherBodyIndex :type Integer))
  (bind _asbp_third_person_character (Utilities|Casting|CastToBP_ThirdPersonCharacter OtherActor))
  (Variables|/Game/ThirdPerson/Blueprints/BP_ThirdPersonCharacter.BP_ThirdPersonCharacter_C|SetBoatDamage _asbp_third_person_character 0)
  (CallFunction|StopRepairing))

(event Custom|DestroyActor
  (bind _asbp_third_person_character (Utilities|Casting|CastToBP_ThirdPersonCharacter (Game|GetPlayerCharacter 0)))
  (Utilities|Array|RemoveItem (Variables|/Game/ThirdPerson/Blueprints/BP_ThirdPersonCharacter.BP_ThirdPersonCharacter_C|GetListBoatDamage _asbp_third_person_character) self)
  (if (Utilities|IsValid (stale OnComponentBeginOverlap(Box) _asbp_companion))
    (Default|ResetVarCompanion (stale OnComponentBeginOverlap(Box) _asbp_companion))
    (Actor|DestroyActor)))

(event Custom|StartRepairing
  (bind _progressbar (Variables|Default|GetProgressBar))
  (Rendering|SetVisibility _progressbar true false)
  (Components|Activation|Activate _progressbar true))

(event Custom|StopRepairing
  (bind _progressbar (Variables|Default|GetProgressBar))
  (Rendering|SetVisibility _progressbar false false)
  (Components|Activation|Deactivate _progressbar))

(event EventBeginPlay
  (bind _returnvalue (Transformation|GetActorLocation))
  (bind _asbp_third_person_character (Utilities|Casting|CastToBP_ThirdPersonCharacter (Game|GetPlayerCharacter 0)))
  (Utilities|Array|Add (Variables|/Game/ThirdPerson/Blueprints/BP_ThirdPersonCharacter.BP_ThirdPersonCharacter_C|GetListBoatDamage _asbp_third_person_character) self)
  (bind _outhit (Collision|LineTraceByChannel _returnvalue (+ _returnvalue (* (Math|Vector|VectorDown) 3e+02)) "TraceTypeQuery1" false 0 "None"))
  (Utilities|Casting|CastToBP_Boat (.hitactor _outhit))
  (Transformation|SetActorLocation (+ (.impactpoint _outhit) "0.000000,0.000000,25.000000") false false)
  (CallFunction|StopRepairing))

(event EventTick
  (params (DeltaSeconds :type Float%20%28single-precision%29))
  (bind _repair_prompt (Variables|Default|GetRepair%20prompt))
  (Transformation|SetWorldRotation _repair_prompt (Math|Rotator|MakeRotator 0.0 0.0 (.yaw (Math|Rotator|FindLookatRotation (Transformation|GetWorldLocation _repair_prompt) (Camera|GetCameraLocation (Game|GetPlayerCameraManager 0))))) false false)
  (if (Components|Activation|IsActive (Variables|Default|GetProgressBar))
    (Transformation|SetWorldRotation (Variables|Default|GetProgressBar) (Math|Rotator|FindLookatRotation (Transformation|GetWorldLocation (Variables|Default|GetProgressBar)) (Camera|GetCameraLocation (Game|GetPlayerCameraManager 0))) false false)))

(fn ConstructionScript)