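; BP_Meteor is a homing meteor projectile that damages boats on contact.
; Tick runs through a one-second Delay, then zeroes rotation so local space matches world space and sets ProjectileMovement velocity toward Target at Speed.
; Overlapping a BP_Boat calls its Damage with the meteor's location and destroys the meteor, while other actors only get their name printed.
; The construction script randomly picks the mesh, though both entries are SM_Meteorite_star.
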(event OnComponentBeginOverlap(BaseMesh)
  (params (OverlappedComponent :type Primitive%20Component%20Object%20Reference) (OtherActor :type Actor%20Object%20Reference) (OtherComp :type Primitive%20Component%20Object%20Reference) (OtherBodyIndex :type Integer) (bFromSweep :type Boolean) (SweepResult :type Hit%20Result%20Structure%20%28by%20ref%29))
  (bind _asbp_boat (Utilities|Casting|CastToBP_Boat OtherActor)
    (:then
      (Default|Damage _asbp_boat (Transformation|GetActorLocation))
      (Development|PrintString "damage spawned")
      (Actor|DestroyActor))
    (:CastFailed
      (Development|PrintString (Utilities|GetDisplayName OtherActor)))))

(event EventTick
  (params (DeltaSeconds :type Float%20%28single-precision%29))
  (bind _target (Variables|Default|GetTarget))
  (Utilities|FlowControl|Delay 1.0)
  (Utilities|IsValid _target
    (:Is%20Valid
      (Development|PrintString "Hello" true true "(R=1.000000,G=0.000000,B=0.368628,A=1.000000)")
      (Transformation|SetActorRotation "0, 0, 0")
      (Game|Components|ProjectileMovement|SetVelocityinLocalSpace (Variables|Default|GetProjectileMovement) (* (Math|Vector|Normalize (- (Transformation|GetActorLocation _target) (Transformation|GetActorLocation))) (Variables|Default|GetSpeed))))))

(fn ConstructionScript
  (Components|StaticMesh|SetStaticMesh (Variables|Default|GetBaseMesh) (.OutItem (Utilities|Array|Random (Utilities|Array|MakeArray "/Game/Mesh/SM_Meteorite_star.SM_Meteorite_star" "/Game/Mesh/SM_Meteorite_star.SM_Meteorite_star")))))