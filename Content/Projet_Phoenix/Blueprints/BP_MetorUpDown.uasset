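; BP_MetorUpDown is an actor, apparently a meteor by its name, that bobs using a sine wave while stepping toward a Target.
; Tick passes through a one-second Delay, so the position updates about once per second while Target is valid.
; The sine offset, timed from BeginPlay, is added to only the Z of the step toward Target.
; That single float becomes the whole location vector, setting all three axes alike without sweeping.
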(event EventTick
  (params (DeltaSeconds :type Float%20%28single-precision%29))
  (bind _returnvalue (Transformation|GetActorLocation))
  (bind _target (Variables|Default|GetTarget))
  (Utilities|FlowControl|Delay 1.0)
  (Utilities|IsValid _target
    (:Is%20Valid
      (Transformation|SetActorLocation (Math|Conversions|ToVector(Float) (+ (* (Math|Trig|Sin(Degrees) (* (- (Utilities|Time|GetGameTimeinSeconds) (Variables|Default|GetStartTime)) (Variables|Default|GetFrequency))) (Variables|Default|GetAmplitude)) (.z (+ (* (Math|Vector|Normalize (- (Transformation|GetActorLocation _target) _returnvalue)) (Variables|Default|GetSpeed)) _returnvalue)))) false false))))

(event EventBeginPlay
  (Variables|Default|SetStartTime (Utilities|Time|GetGameTimeinSeconds)))

(fn ConstructionScript)