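; Blob enemy that fires projectiles when its pawn sensing sees the third-person player character.
; BeginPlay seeds the life widget with current and max health and caches the blob's animation Blueprint.
; Each sighting triggers the attack animation and calls an event that, after a delay, spawns a projectile at the spawn component.
; The blob's own rotation is set only after that spawn, along the projectile-to-player direction.
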(event OnSeePawn(PawnSensing)
  (params (Pawn :type Pawn%20Object%20Reference))
  ;[0.29 0.8073 0.1822] Attack Player
  (bind _asbp_third_person_character (Utilities|Casting|CastToBP_ThirdPersonCharacter Pawn))
  (Variables|Default|SetTargetActor _asbp_third_person_character)
  (CallFunction|ProjectileAction)
  (Default|BlobAttack (Variables|Default|GetAs%20ABP%20Blob)))

(event Custom|ProjectileAction
  ;[0.3968 0.7188 0.1984] Projectile to Attack
  (Utilities|FlowControl|Delay (Variables|Default|GetTimerAttack))
  (bind _returnvalue (Game|SpawnActorfromClass "/Game/Blueprints/BP_ProjectileBlob.BP_ProjectileBlob_C" (Transformation|GetWorldTransform (Variables|Default|GetProjectileSpawnLocation)) "AlwaysSpawn" "MultiplyWithRoot" 0 0))
  (Transformation|SetActorRotation (Math|Rotator|MakeRotfromX (- (Transformation|GetActorLocation (Variables|Default|GetTargetActor)) (Transformation|GetActorLocation _returnvalue)))))

(event EventBeginPlay
  ;[0.4173 1 0.2587] BeginPlay
  (bind _aswbp_ennemi_life (Utilities|Casting|CastToWBP_EnnemiLife (UserInterface|GetWidget (Variables|Default|GetWidget))))
  (Variables|/Game/HUD/WBP_EnnemiLife.WBP_EnnemiLife_C|SetMaxLife _aswbp_ennemi_life (Variables|Default|GetVieMax))
  (Variables|/Game/HUD/WBP_EnnemiLife.WBP_EnnemiLife_C|SetcurrentLife _aswbp_ennemi_life (Variables|Default|GetVie))
  (bind _asabp_blob (Utilities|Casting|CastToABP_blob (Components|SkeletalMesh|GetAnimInstance (Variables|Character|GetMesh))))
  (Variables|Default|SetAs%20ABP%20Blob _asabp_blob))

(fn ConstructionScript)