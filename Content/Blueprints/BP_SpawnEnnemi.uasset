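; Wave spawner that starts at BeginPlay and runs four timed, hard-coded rounds of normal, seagull (Mouette) and blob enemies.
; Each round chains to the next, calling helper events that spawn enemies at preset spots after Delays.
; Normal enemies are flagged IsInBoat and launched toward LandingSpot1 by PhysicAtterissage, using a height- and gravity-based vertical component.
; Back-to-back calls to the same helper hit a pending Delay, so they add no extra spawns.
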(event Custom|SpawnEnnemi%20Normal
  (params (StartLocation :type Vector) (TargetLocation :type Vector))
  ;[0.4656 1 0.3146] SpawnEnnemiNormal
  (Variables|Default|SetStart%20Location StartLocation)
  (Variables|Default|SetTarget%20Location TargetLocation)
  (bind _returnvalue (Game|SpawnActorfromClass "/Game/Blueprints/BP_Ennemi1.BP_Ennemi1_C" (Math|Transform|MakeTransform (Variables|Default|GetStart%20Location) "0, 0, 0" "1.000000,1.000000,1.000000") "Undefined" "MultiplyWithRoot" 0 0))
  (Variables|Default|SetAS%20BP%20Ennemi%201 _returnvalue)
  (if (not (Utilities|Operators|EqualEqual (Variables|Default|GetStart%20Location) (Variables|Default|GetSpawnSpot1) 0.0))
    _
    (else
      (Transformation|SetActorRotation (Variables|Default|GetAS%20BP%20Ennemi%201) "0.000000,180.000000,0.000000")))
  (Utilities|FlowControl|Delay 0.5)
  (Variables|/Game/Blueprints/BP_Ennemi1.BP_Ennemi1_C|SetIsInBoat (Variables|Default|GetAS%20BP%20Ennemi%201) true)
  (CallFunction|PhysicAtterissage (Variables|Default|GetStart%20Location) (Variables|Default|GetTarget%20Location) (Variables|Default|GetAS%20BP%20Ennemi%201)))

(event Custom|SpawnMouette
  (params (StartLocation :type Vector))
  ;[0.3644 0.7865 0.2606] SpawnMouette
  (Game|SpawnActorfromClass "/Game/Blueprints/BP_EnnemiMouette.BP_EnnemiMouette_C" (Math|Transform|MakeTransform StartLocation "0, 0, 0" "1.000000,1.000000,1.000000") "Undefined" "MultiplyWithRoot" 0 0))

(event Custom|2ennemiNormal
  ;[0.4512 1 0.328] Spawn 2ennemi normal
  (Utilities|FlowControl|Delay 2.0)
  (CallFunction|SpawnEnnemiNormal (Variables|Default|GetSpawnSpot1) (Variables|Default|GetLandingSpot1))
  (Utilities|FlowControl|Delay 2.0)
  (CallFunction|SpawnEnnemiNormal (Variables|Default|GetSpawnSpot2) (Variables|Default|GetLandingSpot1)))

(event Custom|SpawnBlob
  (params (StartLocation :type Vector))
  ;[0.1918 1 0.1475] SpawnBlob
  (Game|SpawnActorfromClass "/Game/Blueprints/BP_EnnemiBlob.BP_EnnemiBlob_C" (Math|Transform|MakeTransform StartLocation "0.000000,-90.000000,0.000000" "1.000000,1.000000,1.000000") "Undefined" "MultiplyWithRoot" 0 0))

(event Custom|2ennemiMouette
  ;[0.2089 1 0.1844] 2 ennemi mouette
  (Utilities|FlowControl|Delay 2.0)
  (CallFunction|SpawnMouette (Variables|Default|GetSpawnSpotMouette1))
  (Utilities|FlowControl|Delay 2.0)
  (CallFunction|SpawnMouette (Variables|Default|GetSpawnSpotMouette2)))

(event Custom|blob
  ;[0.4341 1 0.2717] blob
  (Utilities|FlowControl|Delay 2.0)
  (CallFunction|SpawnBlob (Variables|Default|GetSpawnSpotBlob)))

(event Custom|Round1
  ;[0.4585 1 0.3214] Round1
  (CallFunction|2ennemiNormal)
  (Utilities|FlowControl|Delay 5.0)
  (CallFunction|2ennemiMouette)
  (CallFunction|2ennemiMouette)
  (Utilities|FlowControl|Delay 5.0)
  (CallFunction|2ennemiNormal)
  (Utilities|FlowControl|Delay 5.0)
  (CallFunction|Blob)
  (CallFunction|Round2))

(event Custom|Round2
  ;[0.3359 1 0.2436] Round2
  (Development|PrintString "round 2")
  (Utilities|FlowControl|Delay 75.0)
  (CallFunction|2ennemiMouette)
  (CallFunction|2ennemiMouette)
  (CallFunction|2ennemiMouette)
  (CallFunction|2ennemiMouette)
  (Utilities|FlowControl|Delay 5.0)
  (CallFunction|Blob)
  (Utilities|FlowControl|Delay 5.0)
  (CallFunction|2ennemiNormal)
  (CallFunction|2ennemiNormal)
  (CallFunction|Round3))

(event Custom|Round3
  ;[0.4367 1 0.2984] Round3
  (Development|PrintString "round 3")
  (Utilities|FlowControl|Delay 75.0)
  (CallFunction|2ennemiMouette)
  (CallFunction|Blob)
  (Utilities|FlowControl|Delay 5.0)
  (CallFunction|2ennemiNormal)
  (CallFunction|2ennemiNormal)
  (CallFunction|2ennemiNormal)
  (CallFunction|2ennemiNormal)
  (Utilities|FlowControl|Delay 0.2)
  (CallFunction|Blob)
  (CallFunction|Round4))

(event Custom|Round4
  ;[0.4724 1 0.3075] Round4
  (Development|PrintString "round 4")
  (Utilities|FlowControl|Delay 75.0)
  (CallFunction|2ennemiNormal)
  (CallFunction|2ennemiNormal)
  (CallFunction|2ennemiMouette)
  (CallFunction|2ennemiMouette)
  (CallFunction|2ennemiNormal)
  (CallFunction|2ennemiNormal)
  (CallFunction|2ennemiMouette)
  (CallFunction|2ennemiMouette)
  (Utilities|FlowControl|Delay 5.0)
  (CallFunction|Blob)
  (CallFunction|2ennemiNormal)
  (CallFunction|2ennemiNormal)
  (CallFunction|2ennemiMouette)
  (CallFunction|2ennemiMouette)
  (CallFunction|2ennemiNormal)
  (CallFunction|2ennemiNormal)
  (CallFunction|2ennemiMouette)
  (CallFunction|2ennemiMouette)
  (Utilities|FlowControl|Delay 5.0)
  (CallFunction|Blob))

(event EventBeginPlay
  ;[0.5138 1 0.3704] BeginPlay
  (CallFunction|Round1))

(fn ConstructionScript)

(fn PhysicAtterissage
  (params (StartPosition :type Vector) (TargetPosition :type Vector) (Character :type Character%20Object%20Reference))
  (Variables|Default|SetCharacterRef Character)
  (bind _output_get (Variables|Default|SetDirection (Math|Vector|Normalize (- TargetPosition StartPosition))))
  (Development|PrintString (Utilities|String|ToString(Vector) _output_get) true true "(R=0.946885,G=0.989988,B=1.000000,A=1.000000)" 1e+01)
  (bind _output_get_2 (Variables|Default|SetVy (Math|Float|Sqrt (* (Variables|Default|GetLaunchHeight) (Variables|/Script/Engine.CharacterMovementComponent|GetGravityScale (Variables|/Script/Engine.Character|GetCharacterMovement (Variables|Default|GetCharacterRef))) 2.0))))
  (Development|PrintString (Utilities|String|ToString(Float) _output_get_2) true true "(R=0.957051,G=1.000000,B=0.989953,A=1.000000)" 1e+01)
  (bind _output_get_3 (Variables|Default|SetLaunchDirection (Variables|Default|GetDirection)))
  (bind _output_get_4 (Variables|Default|SetLaunchDirection (Math|Vector|MakeVector (.x _output_get_3) (.y _output_get_3) (Variables|Default|GetVy))))
  (Development|PrintString (Utilities|String|ToString(Vector) _output_get_4) true true "(R=0.962442,G=1.000000,B=0.978911,A=1.000000)" 1e+01)
  (Character|LaunchCharacter (Variables|Default|GetCharacterRef) (* (Variables|Default|GetLaunchDirection) (Variables|Default|GetLaunchForce)) true true)
  (Development|PrintString "AfterLaunching")
  (return))