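; BP_Ennemi2 is a ranged enemy that chases and shoots at the player, with a life widget initialized at BeginPlay.
; PawnSensing stores the sighted player as target, but acts only while IsInBoat is true, a flag this graph only sets false.
; FollowPlayer starts an AI move toward the target and triggers a delayed projectile spawn, after which the enemy rotates along the projectile-to-target direction.
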(event OnSeePawn(PawnSensing)
  (params (Pawn :type Pawn%20Object%20Reference))
  ;[0.29 0.8073 0.1822] Go Follow Player
  (bind _asbp_third_person_character (Utilities|Casting|CastToBP_ThirdPersonCharacter Pawn))
  (Variables|Default|SetTargetActor _asbp_third_person_character)
  (if (Variables|Default|GetIsInBoat)
    (CallFunction|FollowPlayer)))

(event Custom|ProjectileAction
  ;[0.3968 0.7188 0.1984] Projectile to Attack
  (Utilities|FlowControl|Delay (Variables|Default|GetTimerAttack))
  (bind _returnvalue (Game|SpawnActorfromClass "/Game/Blueprints/BP_Projectile.BP_Projectile_C" (Transformation|GetWorldTransform (Variables|Default|GetProjectileSpawnLocation)) "AlwaysSpawn" "MultiplyWithRoot" 0 0))
  (Transformation|SetActorRotation (Math|Rotator|MakeRotfromX (- (Transformation|GetActorLocation (Variables|Default|GetTargetActor)) (Transformation|GetActorLocation _returnvalue)))))

(event Custom|FollowPlayer
  ;[0.29 0.8073 0.1822] Go Follow Player
  (CallFunction|ProjectileAction)
  (AI|AIMoveTo self "0, 0, 0" (Variables|Default|GetTargetActor) 2e+02 false))

(event EventBeginPlay
  ;[0.4173 1 0.2587] Set variables de base debut
  (Variables|Default|SetIsInBoat false)
  (bind _aswbp_ennemi_life (Utilities|Casting|CastToWBP_EnnemiLife (UserInterface|GetWidget (Variables|Default|GetWidget))))
  (Variables|/Game/HUD/WBP_EnnemiLife.WBP_EnnemiLife_C|SetMaxLife _aswbp_ennemi_life (Variables|Default|GetVieMax))
  (Variables|/Game/HUD/WBP_EnnemiLife.WBP_EnnemiLife_C|SetcurrentLife _aswbp_ennemi_life (Variables|Default|GetVie)))

(fn ConstructionScript)