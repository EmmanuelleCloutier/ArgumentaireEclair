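; Fish-monster enemy that chases the player and fires projectiles once it sees them and its IsInBoat flag is set.
; BeginPlay clears that flag, passes health values to its life-bar widget and caches the fish animation Blueprint.
; PawnSensing stores the player and calls FollowPlayer, which starts a delayed attack and an AI MoveTo.
; The attack spawns BP_Projectile, turns the enemy using the spawn-to-player direction and triggers the attack animation.
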(event OnSeePawn(PawnSensing)
  (params (Pawn :type Pawn%20Object%20Reference))
  ;[0.29 0.8073 0.1822] Go Follow Player
  (bind _asbp_third_person_character (Utilities|Casting|CastToBP_ThirdPersonCharacter Pawn :!label _label))
  (Utilities|IsValid _asbp_third_person_character
    (:Is%20Valid
      (Variables|Default|SetPlayerReference _asbp_third_person_character)
      (Variables|Default|SetIsSeingPlayer true)
      (if (Variables|Default|GetIsInBoat)
        (CallFunction|FollowPlayer)))
    (:Is%20Not%20Valid
      (Utilities|FlowControl|Delay 0.2)
      (goto _label))))

(event Custom|ProjectileAction
  ;[0.3968 0.7188 0.1984] Projectile to Attack
  (Utilities|FlowControl|Delay (Variables|Default|GetTimerAttack))
  (bind _returnvalue (Game|SpawnActorfromClass "/Game/Blueprints/BP_Projectile.BP_Projectile_C" (Transformation|GetWorldTransform (Variables|Default|GetProjectileSpawnLocation)) "AlwaysSpawn" "MultiplyWithRoot" 0 0))
  (Transformation|SetActorRotation (Math|Rotator|MakeRotfromX (- (Transformation|GetActorLocation (Variables|Default|GetPlayerReference)) (Transformation|GetActorLocation _returnvalue))))
  (Default|Attack (Variables|Default|GetAs%20ABP%20Fish%20Monster)))

(event Custom|FollowPlayer
  ;[0.29 0.8073 0.1822] Go Follow Player
  (if (Variables|Default|GetIsSeingPlayer)
    (CallFunction|ProjectileAction)
    (AI|AIMoveTo self "0, 0, 0" (Variables|Default|GetPlayerReference) 2e+02 false
      (:then
        (Utilities|FlowControl|Delay 5.0)))))

(event EventBeginPlay
  ;[0.4173 1 0.2587] BeginPlay
  (Variables|Default|SetIsInBoat false)
  (bind _aswbp_ennemi_life (Utilities|Casting|CastToWBP_EnnemiLife (UserInterface|GetWidget (Variables|Default|GetWidget))))
  (Variables|/Game/HUD/WBP_EnnemiLife.WBP_EnnemiLife_C|SetMaxLife _aswbp_ennemi_life (Variables|Default|GetVieMax))
  (Variables|/Game/HUD/WBP_EnnemiLife.WBP_EnnemiLife_C|SetcurrentLife _aswbp_ennemi_life (Variables|Default|GetVie))
  (bind _asabp_fish_monster (Utilities|Casting|CastToABP_FishMonster (Components|SkeletalMesh|GetAnimInstance (Variables|Character|GetMesh))))
  (Variables|Default|SetAs%20ABP%20Fish%20Monster _asabp_fish_monster))

(fn ConstructionScript)